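; KGHealthPickup is a pickup actor that restores health to KGCharacterBase characters on overlap.
; It acts only when the character's Health differs from its class default, which serves as the maximum.
; It adds HealthOffering, clamps the result to that class default, and destroys itself, so a character at full health leaves it in place.
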(event `self.ReceiveActorBeginOverlap`
  (params (OtherActor :type "Actor Object Reference"))
  (bind _askgcharacter_base (cast `/Game/Blueprints/KGCharacterBase` OtherActor))
  (bind _health (defaults `/Game/Blueprints/KGHealthPickup` (`GameplayStatics.GetObjectClass` _askgcharacter_base)))
  (if (not (== (`/Game/Blueprints/KGCharacterBase.Health` _askgcharacter_base) _health))
    (set `/Game/Blueprints/KGCharacterBase.Health` (`KismetMathLibrary.FMin` (+ (`/Game/Blueprints/KGCharacterBase.Health` _askgcharacter_base) (`self.HealthOffering`)) _health) _askgcharacter_base)
    (`self.K2_DestroyActor`)))

(fn `UserConstructionScript`)